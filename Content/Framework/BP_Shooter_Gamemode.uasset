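; Shooter game mode that tracks connected player controllers, spawns players and runs the match-start countdown.
; As players join, it reads solo mode and expected player count from the game instance, then restarts controllers at player starts named by their index.
; LevelStart triggers each controller's countdown and enables input after a short delay.
; Logout removes the controller and decrements the expected count.
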(event Custom|LevelStart
  (Utilities|FlowControl|Delay 0.2)
  (for _array_element (Variables|Default|GetAll_ConnectedControllers)
    (Default|GameStartCountDown _array_element))
  (Utilities|FlowControl|Delay 1.0)
  (for _array_element_2 (Variables|Default|GetAll_ConnectedControllers)
    (Default|EnableAllinput _array_element_2)))

(event EventHandleStartingNewPlayer
  (params (NewPlayer :type Player%20Controller%20Object%20Reference))
  (bind _all_connectedcontrollers (Variables|Default|GetAll_ConnectedControllers))
  (bind _output (Utilities|Array|Get(acopy) _all_connectedcontrollers))
  (bind _asbp_shooter_player_controller (Utilities|Casting|CastToBP_Shooter_PlayerController NewPlayer))
  (Utilities|Array|Add (Variables|Default|GetAll_ConnectedControllers) _asbp_shooter_player_controller)
  (bind _asbp_shooter_gameinstance (Utilities|Casting|CastToBP_Shooter_Gameinstance (Game|GetGameInstance)))
  (Variables|Default|SetNum_ExpectedPlayers (Variables|/Game/Framework/BP_Shooter_Gameinstance.BP_Shooter_Gameinstance_C|GetNum%20Connected%20Players _asbp_shooter_gameinstance))
  (if (Variables|/Game/Framework/BP_Shooter_Gameinstance.BP_Shooter_Gameinstance_C|GetIsSoloGame _asbp_shooter_gameinstance)
    (Variables|Default|SetNum_ExpectedPlayers 1)
    (Class|GameModeBase|RestartPlayeratPlayerStart _output (Class|GameModeBase|FindPlayerStart _output "0"))
    (CallFunction|LevelStart)
    (else
      (if (== (Variables|Default|GetNum_ExpectedPlayers) (Utilities|Array|Length (Variables|Default|GetAll_ConnectedControllers)))
        (Utilities|FlowControl|Delay 0.5)
        (else
          (Development|PrintString "PIE launch enabled")))
      (for (_array_element _array_index) (Variables|Default|GetAll_ConnectedControllers)
        (Class|GameModeBase|RestartPlayeratPlayerStart _array_element (Class|GameModeBase|FindPlayerStart _array_element (Utilities|String|ToString(Integer) _array_index))))
      (CallFunction|LevelStart))))

(event EventOnLogout
  (params (ExitingController :type Controller%20Object%20Reference))
  (bind _asbp_shooter_player_controller (Utilities|Casting|CastToBP_Shooter_PlayerController ExitingController))
  (Utilities|Array|RemoveItem (Variables|Default|GetAll_ConnectedControllers) _asbp_shooter_player_controller)
  (Math|Integer|DecrementInt (Variables|Default|GetNum_ExpectedPlayers)))

(fn ConstructionScript)