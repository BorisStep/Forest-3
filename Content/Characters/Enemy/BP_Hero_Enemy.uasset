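; Networked shooter hero character, filed as an enemy, with aiming, firing, reload, dash and weapon switching; possession disables player input.
; Input routes through server RPCs and multicasts for montages, effects and dash impulses.
; A three-slot inventory pulls fire stats, meshes, effects and animations from a weapon data table.
; Shots trace from camera, then muzzle, with shotgun spread, but only draw debug lines; several other inputs just print placeholder text.
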(event Custom|Server_SetIsAds
  (params (IsADS :type Boolean))
  ;[1 1 1] IA_Ads
  (Variables|Default|SetIsADS IsADS))

(event Custom|DisableAllInput
  (params (PlayerController :type Player%20Controller%20Object%20Reference))
  (Input|DisableInput PlayerController))

(event Custom|MulticastReloadMontage
  (Animation|Montage|PlayMontage (Variables|Character|GetMesh) (Variables|Default|GetChar%20Reload%20Montage)
    (:then
      (Components|Animation|PlayAnimation (Variables|Default|GetWeaponMesh) (Variables|Default|GetWpn%20Reload%20Anim) false))
    (:OnCompleted
      (Variables|Default|SetIsReloading false))))

(event Custom|Ability_Dash
  (params (Direction :type E_CharMoveDirection%20Enum :default "NewEnumerator0"))
  (Networking|SwitchHasAuthority
    (:Authority
      (CallFunction|MulticastAbilityDash Direction))
    (:Remote
      (CallFunction|ServerAbilityDash Direction))))

(event Custom|Server_Ability_Dash
  (params (Direction :type E_CharMoveDirection%20Enum :default "NewEnumerator0"))
  (CallFunction|MulticastAbilityDash Direction))

(event Custom|Multicast_Ability_Dash
  (params (Direction :type E_CharMoveDirection%20Enum :default "NewEnumerator0"))
  (Default|PlayDashMontage (Variables|Default|GetAnimationInstance) Direction)
  (if (Networking|IsServer)
    (CallFunction|ServerAddDashImpulse Direction)))

(event Custom|DashCooldown
  (Utilities|FlowControl|Delay 1.0)
  (Variables|Default|SetIsDashing false))

(event Custom|Server_SelectWeapon
  (params (InventoryIndex :type Integer))
  (CallFunction|ServerSetReplicatedWpnVars InventoryIndex)
  (CallFunction|MCSelectWeapon (Utilities|Array|Get(acopy) (Variables|Default|GetWeaponInventoryNames) InventoryIndex)))

(event Custom|MC_SelectWeapon
  (params (WeaponRowName :type Name))
  (CallFunction|SetWeaponsCosmetics WeaponRowName))

(event Custom|SwitchWeapon
  (params (InventoryIndex :type Integer))
  (Networking|SwitchHasAuthority
    (:Authority
      (CallFunction|MCSwitchWeapon InventoryIndex))
    (:Remote
      (CallFunction|ServerSwitchWeapon InventoryIndex))))

(event Custom|Server_SwitchWeapon
  (params (InventoryIndex :type Integer))
  (CallFunction|MCSwitchWeapon InventoryIndex))

(event Custom|MC_SwitchWeapon
  (params (InventoryIndex :type Integer))
  (if (== (Utilities|Array|Get(acopy) (Variables|Default|GetWeaponInventoryNames) InventoryIndex) "Pistol")
    (Variables|Default|SetCharEquipMontage "/Game/Characters/Heroes/Mannequin/Animations/Actions/MM_Pistol_Equip_Montage.MM_Pistol_Equip_Montage")
    (else
      (Variables|Default|SetCharEquipMontage "/Game/Characters/Heroes/Mannequin/Animations/Actions/MM_Rifle_Equip_Montage.MM_Rifle_Equip_Montage")))
  (Animation|Montage|PlayMontage (Variables|Character|GetMesh) (Variables|Default|GetCharEquipMontage)
    (:then
      (if (Networking|IsServer)
        (Utilities|FlowControl|Delay 0.4)
        (CallFunction|ServerSelectWeapon InventoryIndex)))
    (:OnBlendOut
      (Variables|Default|SetIsSwitchingWeapon false :!label _label))
    (:OnInterrupted
      (goto _label))))

(event Custom|Server_FireWeapon
  ;[1 1 1] IA_Fire Weapon
  (Variables|Default|SetIsFiring true)
  (Variables|Default|SetIsFireButtonPressed true)
  (CallFunction|ServerBulletTrace :!label _label)
  (CallFunction|ServerFireWeaponEvents)
  (Utilities|FlowControl|Delay (Variables|Default|GetFire%20Time))
  (if (and (Variables|Default|GetIs%20Auto%20Rifle) (Variables|Default|GetIsFireButtonPressed))
    (goto _label)
    (else
      (Variables|Default|SetIsFiring false)
      (Variables|Default|SetIsFireButtonPressed false))))

(event Custom|StopFireWeapon
  ;[1 1 1] IA_Fire Weapon
  (Variables|Default|SetIsFireButtonPressed false))

(event Custom|Server_FireWeaponEvents
  ;[1 1 1] IA_Fire Weapon
  (Utilities|FlowControl|Sequence
    (:then_0
      (CallFunction|MulticastFireMontage))
    (:then_1
      (CallFunction|MCPlayFireSound))
    (:then_2
      (CallFunction|MCMuzzleFlash))))

(event Custom|MC_PlayFireSound
  (Audio|PlaySoundatLocation (Variables|Default|GetFire%20Sound) (Transformation|GetWorldLocation (Variables|Default|GetWeaponMesh)) "0, 0, 0" 0.3 1.0 0.0 0 0 0 0))

(event Custom|MC_MuzzleFlash
  (Effects|SpawnEmitterAttached (Variables|Default|GetMuzzle%20Flash%20FX) (Variables|Default|GetWeaponMesh) (Variables|Default|GetMuzzle%20Socket) "0, 0, 0" "0, 0, 0" "1.000000,1.000000,1.000000" "SnapToTarget"))

(event Custom|UpdateMoveState
  (params (IsMovingThisFrame :type Boolean))
  (if (!= IsMovingThisFrame (Variables|Default|GetIsMoving))
    (Variables|Default|SetIsMoving IsMovingThisFrame)
    (Networking|SwitchHasAuthority
      (:Authority
        (Variables|/Script/Engine.CharacterMovementComponent|SetbUseControllerDesiredRotation (Variables|Character|GetCharacterMovement) (Variables|Default|GetIsMoving)))
      (:Remote
        (CallFunction|ServerSetUseDeisredRot (Variables|Default|GetIsMoving))
        (Variables|/Script/Engine.CharacterMovementComponent|SetbUseControllerDesiredRotation (Variables|Character|GetCharacterMovement) (Variables|Default|GetIsMoving))))
    (else
      (Variables|Default|SetIsMoving IsMovingThisFrame))))

(event Custom|Server_SetUseDeisredRot
  (params (Use%20Controller%20Desired%20Rotation :type Boolean))
  (Variables|/Script/Engine.CharacterMovementComponent|SetbUseControllerDesiredRotation (Variables|Character|GetCharacterMovement) Use%20Controller%20Desired%20Rotation))

(event Custom|Sever_SetAimRotation
  (params (AimRotation :type Rotator))
  (Variables|Default|SetAimRotation AimRotation))

(event Custom|MulticastFireMontage
  (Animation|Montage|PlayMontage (Variables|Character|GetMesh) (Variables|Default|GetChar%20Fire%20Montage)
    (:then
      (Components|Animation|PlayAnimation (Variables|Default|GetWeaponMesh) (Variables|Default|GetWpn%20Fire%20Anim) false))))

(event Custom|PlayReloadMontage
  (Networking|SwitchHasAuthority
    (:Authority
      (CallFunction|MulticastReloadMontage))
    (:Remote
      (CallFunction|ServerReloadMontage))))

(event Custom|ServerReloadMontage
  (CallFunction|MulticastReloadMontage))

(event Input|EnhancedActionEvents|EnhancedInputActionIA_Look
  (params (ActionValue :type Vector%202D%20Structure) (ElapsedSeconds :type Float%20%28double-precision%29) (TriggeredSeconds :type Float%20%28double-precision%29) (InputAction :type Input%20Action%20Object%20Reference :default "/Game/Input/Actions/IA_Look.IA_Look"))
  ;[1 1 1] IA_Look
  (:Triggered
    (Pawn|Input|AddControllerYawInput (.x ActionValue))
    (Pawn|Input|AddControllerPitchInput (.y ActionValue))))

(event Input|EnhancedActionEvents|EnhancedInputActionIA_Move
  (params (ActionValue :type Vector%202D%20Structure) (ElapsedSeconds :type Float%20%28double-precision%29) (TriggeredSeconds :type Float%20%28double-precision%29) (InputAction :type Input%20Action%20Object%20Reference :default "/Game/Input/Actions/IA_Move.IA_Move"))
  (bind _returnvalue (Pawn|GetControlRotation :!class /Script/Engine.Pawn))
  ;[1 1 1] IA_Move
  (:Triggered
    (Pawn|Input|AddMovementInput (Math|Vector|GetRightVector (Math|Rotator|MakeRotator (.roll _returnvalue) 0.0 (.yaw _returnvalue))) (.x ActionValue) false)
    (Pawn|Input|AddMovementInput (Math|Vector|GetForwardVector (Math|Rotator|MakeRotator 0.0 0.0 (.yaw (Pawn|GetControlRotation :!class /Script/Engine.Pawn)))) (.y ActionValue) false)))

(event Input|EnhancedActionEvents|EnhancedInputActionIA_SwitchShould
  (params (ActionValue :type Boolean) (ElapsedSeconds :type Float%20%28double-precision%29) (TriggeredSeconds :type Float%20%28double-precision%29) (InputAction :type Input%20Action%20Object%20Reference :default "/Game/Input/Actions/IA_SwitchShould.IA_SwitchShould"))
  (:Started
    (Development|PrintString "Hello"))
  (:Completed
    (Development|PrintString "Hello")))

(event Input|EnhancedActionEvents|EnhancedInputActionIA_Jump
  (params (ActionValue :type Boolean) (ElapsedSeconds :type Float%20%28double-precision%29) (TriggeredSeconds :type Float%20%28double-precision%29) (InputAction :type Input%20Action%20Object%20Reference :default "/Game/Input/Actions/IA_Jump.IA_Jump"))
  (:Triggered
    (Development|PrintString "Hello"))
  (:Completed
    (Development|PrintString "Hello")))

(event Input|EnhancedActionEvents|EnhancedInputActionIA_Crouch
  (params (ActionValue :type Boolean) (ElapsedSeconds :type Float%20%28double-precision%29) (TriggeredSeconds :type Float%20%28double-precision%29) (InputAction :type Input%20Action%20Object%20Reference :default "/Game/Input/Actions/IA_Crouch.IA_Crouch"))
  (:Started
    (Development|PrintString "Hello"))
  (:Completed
    (Development|PrintString "Hello")))

(event Input|EnhancedActionEvents|EnhancedInputActionIA_Melee
  (params (ActionValue :type Boolean) (ElapsedSeconds :type Float%20%28double-precision%29) (TriggeredSeconds :type Float%20%28double-precision%29) (InputAction :type Input%20Action%20Object%20Reference :default "/Game/Input/Actions/IA_Melee.IA_Melee"))
  (:Started
    (Development|PrintString "Hello"))
  (:Completed
    (Development|PrintString "Hello")))

(event Input|EnhancedActionEvents|EnhancedInputActionIA_ThrowGrenade
  (params (ActionValue :type Boolean) (ElapsedSeconds :type Float%20%28double-precision%29) (TriggeredSeconds :type Float%20%28double-precision%29) (InputAction :type Input%20Action%20Object%20Reference :default "/Game/Input/Actions/IA_ThrowGrenade.IA_ThrowGrenade"))
  (:Started
    (Development|PrintString "Hello"))
  (:Completed
    (Development|PrintString "Hello")))

(event Input|EnhancedActionEvents|EnhancedInputActionIA_ToggleInventory
  (params (ActionValue :type Boolean) (ElapsedSeconds :type Float%20%28double-precision%29) (TriggeredSeconds :type Float%20%28double-precision%29) (InputAction :type Input%20Action%20Object%20Reference :default "/Game/Input/Actions/IA_ToggleInventory.IA_ToggleInventory"))
  (:Started
    (Development|PrintString "Hello"))
  (:Completed
    (Development|PrintString "Hello")))

(event Input|EnhancedActionEvents|EnhancedInputActionIA_ADS
  (params (ActionValue :type Boolean) (ElapsedSeconds :type Float%20%28double-precision%29) (TriggeredSeconds :type Float%20%28double-precision%29) (InputAction :type Input%20Action%20Object%20Reference :default "/Game/Input/Actions/IA_ADS.IA_ADS"))
  ;[1 1 1] IA_Ads
  (:Started
    (Networking|SwitchHasAuthority
      (:Authority
        _)
      (:Remote
        (CallFunction|ServerSetIsAds true)))
    (Variables|Default|SetIsADS true))
  (:Completed
    (Networking|SwitchHasAuthority
      (:Authority
        _)
      (:Remote
        (CallFunction|ServerSetIsAds false)))
    (Variables|Default|SetIsADS false)))

(event Input|EnhancedActionEvents|EnhancedInputActionIA_FireWeapon
  (params (ActionValue :type Boolean) (ElapsedSeconds :type Float%20%28double-precision%29) (TriggeredSeconds :type Float%20%28double-precision%29) (InputAction :type Input%20Action%20Object%20Reference :default "/Game/Input/Actions/IA_FireWeapon.IA_FireWeapon"))
  ;[1 1 1] IA_Fire Weapon
  (:Started
    (if (not (Variables|Default|GetIsFiring))
      (CallFunction|ServerFireWeapon)))
  (:Completed
    (CallFunction|StopFireWeapon)))

(event Input|EnhancedActionEvents|EnhancedInputActionIA_PauseGame
  (params (ActionValue :type Boolean) (ElapsedSeconds :type Float%20%28double-precision%29) (TriggeredSeconds :type Float%20%28double-precision%29) (InputAction :type Input%20Action%20Object%20Reference :default "/Game/Input/Actions/IA_PauseGame.IA_PauseGame"))
  ;[1 1 1] Pause
  (:Started
    (bind _asbp_shooter_gameinstance (Utilities|Casting|CastToBP_Shooter_Gameinstance (Game|GetGameInstance)))
    (bind _isgamepausedresult (Default|TogglePauseGame _asbp_shooter_gameinstance))
    (if _isgamepausedresult
      (Widget|SetVisibility (Variables|Default|GetWB%20Ingame%20HUD) "Hidden")
      (else
        (Widget|SetVisibility (Variables|Default|GetWB%20Ingame%20HUD) "Visible")))))

(event Input|EnhancedActionEvents|EnhancedInputActionIA_Reload
  (params (ActionValue :type Boolean) (ElapsedSeconds :type Float%20%28double-precision%29) (TriggeredSeconds :type Float%20%28double-precision%29) (InputAction :type Input%20Action%20Object%20Reference :default "/Game/Input/Actions/IA_Reload.IA_Reload"))
  ;[1 1 1] Reload
  (:Started
    (if (not (Variables|Default|GetIsReloading))
      (Variables|Default|SetIsReloading true)
      (CallFunction|PlayReloadMontage))))

(event Input|EnhancedActionEvents|EnhancedInputActionIA_Dash
  (params (ActionValue :type Boolean) (ElapsedSeconds :type Float%20%28double-precision%29) (TriggeredSeconds :type Float%20%28double-precision%29) (InputAction :type Input%20Action%20Object%20Reference :default "/Game/Input/Actions/IA_Dash.IA_Dash"))
  ;[1 1 1] Dash
  (:Started
    (bind _candash (CallFunction|CanDash))
    (if _candash
      (Variables|Default|SetIsDashing true)
      (CallFunction|AbilityDash (Variables|/Game/Characters/ABP_Hero_Quin.ABP_Hero_Quin_C|GetMoveDirection (Variables|Default|GetAnimationInstance)))
      (CallFunction|DashCooldown))))

(event Input|EnhancedActionEvents|EnhancedInputActionIA_SwitchWeapon
  (params (ActionValue :type Boolean) (ElapsedSeconds :type Float%20%28double-precision%29) (TriggeredSeconds :type Float%20%28double-precision%29) (InputAction :type Input%20Action%20Object%20Reference :default "/Game/Input/Actions/IA_SwitchWeapon.IA_SwitchWeapon"))
  ;[1 1 1] Switch Weapon
  (:Started
    (if (not (Variables|Default|GetIsSwitchingWeapon))
      (Variables|Default|SetIsSwitchingWeapon true)
      (if (== (Variables|Default|GetActiveWeaponIndex) (- (Utilities|Array|Length (Variables|Default|GetWeaponInventoryNames)) 1))
        (CallFunction|SwitchWeapon)
        (else
          (CallFunction|SwitchWeapon (+ (Variables|Default|GetActiveWeaponIndex) 1)))))))

(event Input|EnhancedActionEvents|EnhancedInputActionIA_Interact
  (params (ActionValue :type Boolean) (ElapsedSeconds :type Float%20%28double-precision%29) (TriggeredSeconds :type Float%20%28double-precision%29) (InputAction :type Input%20Action%20Object%20Reference :default "/Game/Input/Actions/IA_Interact.IA_Interact"))
  (:Completed
    (Development|PrintString "Hello")))

(event Input|EnhancedActionEvents|EnhancedInputActionIA_ToggleScoreBoard
  (params (ActionValue :type Boolean) (ElapsedSeconds :type Float%20%28double-precision%29) (TriggeredSeconds :type Float%20%28double-precision%29) (InputAction :type Input%20Action%20Object%20Reference :default "/Game/Input/Actions/IA_ToggleScoreBoard.IA_ToggleScoreBoard"))
  (:Started
    (Development|PrintString "Hello"))
  (:Completed
    (Development|PrintString "Hello")))

(event EventBeginPlay
  (if (Pawn|IsLocallyControlled)
    (bind _asbp_shooter_player_controller (Utilities|Casting|CastToBP_Shooter_PlayerController (Game|GetPlayerController 0)))
    (Variables|Default|SetWB%20Ingame%20HUD (Variables|/Game/Framework/BP_Shooter_PlayerController.BP_Shooter_PlayerController_C|GetWB_IngameHUD _asbp_shooter_player_controller))
    (else
      (Actor|Tick|SetActorTickEnabled false)))
  (bind _asabp_hero_quin (Utilities|Casting|CastToABP_Hero_Quin (Components|SkeletalMesh|GetAnimInstance (Variables|Character|GetMesh))))
  (Variables|Default|SetAnimationInstance _asabp_hero_quin)
  (if (Networking|IsServer)
    (Utilities|FlowControl|Delay 2.0)
    (CallFunction|ServerAddWpntoInventory 0 "Pistol")
    (CallFunction|ServerAddWpntoInventory 1 "AssaultRifle")
    (CallFunction|ServerAddWpntoInventory 2 "Shotgun")
    (CallFunction|ServerSelectWeapon)))

(event EventTick
  (params (DeltaSeconds :type Float%20%28single-precision%29))
  (CallFunction|UpdateMoveState (> (Math|Vector|VectorLengthXY (Transformation|GetVelocity)) 0.0))
  (Variables|Default|SetNew_AimRotation (Pawn|GetBaseAimRotation))
  (Networking|SwitchHasAuthority
    (:Authority
      (Variables|Default|SetAimRotation (Variables|Default|GetNew_AimRotation)))
    (:Remote
      (CallFunction|SeverSetAimRotation (Variables|Default|GetNew_AimRotation))
      (Variables|Default|SetAimRotation (Variables|Default|GetNew_AimRotation)))))

(event EventPossessed
  (params (NewController :type Controller%20Object%20Reference))
  (CallFunction|DisableAllInput (.AsPlayer%20Controller (Utilities|Casting|CastToPlayerController NewController))))

(fn ConstructionScript)

(fn CanDash
  (if (and (not (Variables|Default|GetIsDashing)) (not (Variables|/Game/Characters/ABP_Hero_Quin.ABP_Hero_Quin_C|GetIsPlayingTurnMontage (Variables|Default|GetAnimationInstance))))
    (return true)
    (else
      (return false))))

(fn ServerAddDashImpulse
  (params (Direction :type E_CharMoveDirection%20Enum :default "NewEnumerator0"))
  (switch Utilities|FlowControl|Switch|SwitchonE_CharMoveDirection Direction
    (:NewEnumerator0
      (LocalVariables|SetLcl_Impulse (* (Transformation|GetActorForwardVector) 1000) :!label _label))
    (:NewEnumerator1
      (goto _label))
    (:NewEnumerator2
      (LocalVariables|SetLcl_Impulse (* (Transformation|GetActorForwardVector) -1000)))
    (:NewEnumerator3
      (LocalVariables|SetLcl_Impulse (* (Transformation|GetActorRightVector) -1000)))
    (:NewEnumerator4
      (LocalVariables|SetLcl_Impulse (* (Transformation|GetActorRightVector) 1000))))
  (LocalVariables|SetLcl_Impulse (+ (LocalVariables|GetLcl_Impulse) "0.000000,0.000000,250.000000"))
  (Physics|AddImpulse (Variables|Character|GetCharacterMovement) (LocalVariables|GetLcl_Impulse) true)
  (return))

(fn ServerAddWpntoInventory
  (params (InventorySlot :type Integer) (WeaponRowName :type Name))
  (Utilities|Array|SetArrayElem (Variables|Default|GetWeaponInventoryNames) InventorySlot WeaponRowName true)
  (return))

(fn ServerSetReplicatedWpnVars
  (params (InventoryIndex :type Integer))
  (Variables|Default|SetActiveWeaponIndex InventoryIndex)
  (bind _returnvalue (Utilities|GetDataTableRow "/Game/Weapons/WeaponInfo_Table.WeaponInfo_Table" (Utilities|Array|Get(acopy) (Variables|Default|GetWeaponInventoryNames) InventoryIndex))
    (:then
      (Variables|Default|SetFire%20Time (.FireTime (Utilities|Struct|BreakS_WeaponInfo _returnvalue)))
      (Variables|Default|SetIs%20Auto%20Rifle (.IsAutoRifle (Utilities|Struct|BreakS_WeaponInfo _returnvalue)))
      (Variables|Default|SetIs%20Shotgun (.IsShotgun (Utilities|Struct|BreakS_WeaponInfo _returnvalue)))
      (return))))

(fn SetWeaponsCosmetics
  (params (WeaponRowName :type Name))
  (bind _animationinstance (Variables|Default|GetAnimationInstance))
  (bind _returnvalue (Utilities|GetDataTableRow "/Game/Weapons/WeaponInfo_Table.WeaponInfo_Table" WeaponRowName)
    (:then
      (Components|SkeletalMesh|SetSkeletalMeshAsset (Variables|Default|GetWeaponMesh) (.WeaponMesh (Utilities|Struct|BreakS_WeaponInfo _returnvalue)))
      (Variables|Default|SetFire%20Sound (.FireSound (Utilities|Struct|BreakS_WeaponInfo _returnvalue)))
      (Variables|Default|SetMuzzle%20Socket (.MuzzleSocket (Utilities|Struct|BreakS_WeaponInfo _returnvalue)))
      (Variables|Default|SetShell%20Eject%20Socket (.ShellEjectSocket (Utilities|Struct|BreakS_WeaponInfo _returnvalue)))
      (Variables|Default|SetWpn%20Fire%20Anim (.Wpn_FireAnim (Utilities|Struct|BreakS_WeaponInfo _returnvalue)))
      (Variables|Default|SetWpn%20Reload%20Anim (.Wpn_ReloadAnim (Utilities|Struct|BreakS_WeaponInfo _returnvalue)))
      (Variables|Default|SetChar%20Fire%20Montage (.Char_FireMontage (Utilities|Struct|BreakS_WeaponInfo _returnvalue)))
      (Variables|Default|SetChar%20Reload%20Montage (.Char_ReloadMontage (Utilities|Struct|BreakS_WeaponInfo _returnvalue)))
      (Variables|Default|SetMuzzle%20Flash%20FX (.MuzzleFlash_FX (Utilities|Struct|BreakS_WeaponInfo _returnvalue)))
      (Variables|/Game/Characters/ABP_Hero_Quin.ABP_Hero_Quin_C|SetChar_Ads_Idle _animationinstance (.Char_ADS_idle (Utilities|Struct|BreakS_WeaponInfo _returnvalue)))
      (Variables|/Game/Characters/ABP_Hero_Quin.ABP_Hero_Quin_C|SetChar_Hip_Idle _animationinstance (.Char_Hip_Idle (Utilities|Struct|BreakS_WeaponInfo _returnvalue)))
      (Variables|/Game/Characters/ABP_Hero_Quin.ABP_Hero_Quin_C|SetChar_ADS_AO _animationinstance (.Char_ADS_AO (Utilities|Struct|BreakS_WeaponInfo _returnvalue)))
      (Variables|/Game/Characters/ABP_Hero_Quin.ABP_Hero_Quin_C|SetChar_Hip_AO _animationinstance (.Char_Hip_AO (Utilities|Struct|BreakS_WeaponInfo _returnvalue)))
      (return))))

(fn ServerBulletTrace
  (bind _camera (Variables|Default|GetCamera))
  (bind _weaponmesh (Variables|Default|GetWeaponMesh))
  (bind _muzzle_socket (Variables|Default|GetMuzzle%20Socket))
  (bind _weaponmesh_2 (Variables|Default|GetWeaponMesh))
  (bind _muzzle_socket_2 (Variables|Default|GetMuzzle%20Socket))
  (bind _returnvalue (Transformation|GetWorldTransform _camera))
  (bind _returnvalue_2 (Transformation|GetSocketLocation _weaponmesh _muzzle_socket))
  (bind _returnvalue_3 (Transformation|GetSocketLocation _weaponmesh_2 _muzzle_socket_2))
  (bind (_outhit _returnvalue_4) (Collision|LineTraceByChannel (.location _returnvalue) (+ (.location _returnvalue) (* (Math|Vector|GetForwardVector (.rotation _returnvalue)) 100000)) "TraceTypeQuery1" false 0 "None"))
  (if _returnvalue_4
    (LocalVariables|SetLcl_TargetLocation (.Location (Collision|BreakHitResult _outhit)))
    (else
      (LocalVariables|SetLcl_TargetLocation (.TraceEnd (Collision|BreakHitResult _outhit)))))
  (if (Variables|Default|GetIs%20Shotgun)
    (Math|Integer|IncrementInt (LocalVariables|GetLcl_ShotgunShot) :!label _label
      (:%20%20
        (Collision|LineTraceByChannel _returnvalue_2 (+ _returnvalue_2 (* (Math|Random|RandomUnitVectorinConeinDegrees (Math|Vector|GetUnitDirection(Vector) _returnvalue_2 (LocalVariables|GetLcl_TargetLocation)) 3.0) 100000)) "TraceTypeQuery1" false 0 "ForDuration")
        (if (< (LocalVariables|GetLcl_ShotgunShot) 8)
          (goto _label)
          (else
            _))))
    (else
      (Collision|LineTraceByChannel _returnvalue_3 (+ _returnvalue_3 (* (Math|Vector|GetUnitDirection(Vector) _returnvalue_3 (LocalVariables|GetLcl_TargetLocation)) 100000)) "TraceTypeQuery1" false 0 "ForDuration")))
  (return))